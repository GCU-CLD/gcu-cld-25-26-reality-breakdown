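; Base enemy character with patrol helpers, optional pistol, shooting, a player-killing tackle and reset to spawn state.
; Each tick, two box traces along X in the facing direction detect standing or crouching players and update detection status.
; Sight changes switch behaviour to chase, shoot or default through the AI controller, which also receives the spotted player.
; Tackling plays paired montages, using motion warping to align both characters before the player dies.
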(event Custom|ForceMantle
  ;[1 1 1] Force Mantle if walking into a Mantle Zone
  (CallFunction|Mantle false (.1mMantle (CallFunction|GetNearestMantleSpot))))

(event Custom|TacklePlayer
  (bind _returnvalue (Game|GetPlayerCharacter 0))
  (bind _asbp_player_character (Utilities|Casting|CastToBP_PlayerCharacter _returnvalue))
  (bind _currentlycarriedobject (Variables|/Game/PGTemplate/Blueprints/Characters/Core/BP_PlatformGameCharacter.BP_PlatformGameCharacter_C|GetCurrentlyCarriedObject _asbp_player_character))
  ;[1 1 1] Tackle by playintg the animation on both yourself and the player
  (if (> (Variables|Default|GetHealth) 0.0)
    (AI|RunBehaviorTree (AI|GetAIController self))
    (Variables|Default|SetTackling true)
    (Collision|SetCollisionEnabled (Variables|Default|GetCapsuleComponent) "NoCollision")
    (Animation|PlayAnimMontage "/Game/PGTemplate/Blueprints/Characters/Core/Animations/Mixamo/Enemies/DoubleLegTakedownAttacker_UE_Montage.DoubleLegTakedownAttacker_UE_Montage" 1.0 "None")
    (Collision|SetCollisionEnabled (Variables|/Script/Engine.Character|GetCapsuleComponent _returnvalue) "NoCollision")
    (Class|MotionWarpingComponent|AddorUpdateWarpTarget (Variables|/Game/PGTemplate/Blueprints/Characters/Player/BP_PlayerCharacter.BP_PlayerCharacter_C|GetMotionWarping _asbp_player_character) (Utilities|Struct|MakeMotionWarpingTarget "EnemyPosition" "0.000000,0.000000,0.000000" "0.000000,0.000000,0.000000" (Variables|Character|GetMesh) "None" true))
    (Utilities|IsValid _currentlycarriedobject
      (:Is%20Valid
        (Default|Drop _currentlycarriedobject _asbp_player_character))
      (:Is%20Not%20Valid
        _))
    (bind _returnvalue_2 (Animation|PlayAnimMontage _returnvalue (select (CallFunction|IsFacingTowardsPlayer) "/Game/PGTemplate/Blueprints/Characters/Core/Animations/Mixamo/Enemies/DoubleLegTakedownVictim_UE_Montage.DoubleLegTakedownVictim_UE_Montage" "/Game/PGTemplate/Blueprints/Characters/Core/Animations/Mixamo/Enemies/Tripping_UE_Montage.Tripping_UE_Montage") 1.0 "None"))
    (Utilities|FlowControl|Delay _returnvalue_2)
    (bind _asbp_player_character_2 (Utilities|Casting|CastToBP_PlayerCharacter (Game|Player|GetPlayerPawn 0)))
    (Default|Die _asbp_player_character_2)))

(event Custom|ReactToPlayer
  (params (Player :type BP%20Player%20Character%20Object%20Reference))
  ;[1 1 1] React To Player
  (Animation|PlayAnimMontage "/Game/PGTemplate/Blueprints/Characters/Core/Animations/Mixamo/Enemies/Reacting_UE_Montage.Reacting_UE_Montage" 1.0 "None"))

(event Custom|CancelBehaviour
  ;[1 1 1] Tick Actions
  ;;[0 0 0] State based Behaviour
  (Utilities|FlowControl|Sequence
    (:then_0
      (|IdleBehaviour) ; enters at CancelBehaviour
    )
    (:then_1
      (|PatrollingBehaviour) ; enters at CancelBehaviour
    )
    (:then_2
      (|ChasingBehaviour) ; enters at CancelBehaviour
    )))

(event Custom|Shoot
  (bind _self self)
  (bind _playerdetectionstatus (Variables|Default|GetPlayerDetectionStatus))
  (bind _gunmesh (Variables|Default|GetGunMesh))
  (bind _returnvalue (Transformation|GetActorLocation (.lastspottedplayer _playerdetectionstatus)))
  (bind _returnvalue_2 (Transformation|GetSocketLocation _gunmesh "MuzzleFlash"))
  ;[1 1 1] Shoot
  (Utilities|IsValid (.lastspottedplayer (Variables|Default|GetPlayerDetectionStatus))
    (:Is%20Valid
      (Animation|StopAnimMontage 0)
      (Utilities|FlowControl|Delay 0.5)
      (Transformation|SetActorRotation (Math|Rotator|MakeRotator 0.0 0.0 (Math|Float|SelectFloat 0.0 1.8e+02 (CallFunction|IsFacingRight))))
      (Animation|Montage|PlayMontage (Variables|Character|GetMesh) "/Game/PGTemplate/Blueprints/Characters/Core/Animations/PistolStarterPack/W1_Stand_Fire_Single_Montage.W1_Stand_Fire_Single_Montage"
        (:then
          (Components|Animation|PlayAnimation _gunmesh "/Game/PGTemplate/Blueprints/Characters/Enemy/PrototypeWeaponsPack/Mesh/PistolFiring_Anim_Slide_SlideAction_002.PistolFiring_Anim_Slide_SlideAction_002" false)
          (Components|Activation|Activate (Variables|Default|GetPistolFire_NS) true)
          (Utilities|IsValid (.lastspottedplayer _playerdetectionstatus)
            (:Is%20Valid
              (Game|SpawnActorfromClass "/Game/PGTemplate/Blueprints/Characters/Enemy/PrototypeWeaponsPack/Mesh/PistolProjectile_BP.PistolProjectile_BP_C" (Math|Transform|MakeTransform _returnvalue_2 (Math|Rotator|FindLookatRotation _returnvalue_2 (Math|Vector|MakeVector (.x _returnvalue) (.y _returnvalue) (.Z (Math|Vector|BreakVector _returnvalue_2)))) "1.000000,1.000000,1.000000") "Undefined" "MultiplyWithRoot" 0 _self (Variables|Default|GetDamageDoneWhenShooting) 1e+01 _self))))))))

(event EventOnReset
  (CallFunction|StopRagdolling)
  (Transformation|SetActorTransform (Variables|Default|GetStartingTransform) false true)
  (CallFunction|SetBehaviour (Variables|Default|GetDefaultBehaviour))
  (Variables|Default|SetHealth 0.1)
  ;[1 1 1] BeginPlay Actions
  (Variables|Default|SetCurrentNode (Variables|Default|GetStartingNode))
  (bind _asenemy_aicontroller_aic (Utilities|Casting|CastToEnemy_AIController_AIC (Pawn|GetController)))
  (Variables|Default|SetAI_Controller _asenemy_aicontroller_aic)
  (CallFunction|SetBehaviour (Variables|Default|GetDefaultBehaviour))
  (Variables|Default|SetStartingTransform (Transformation|GetActorTransform))
  (Variables|Default|SetHealth 0.1)
  (Variables|Default|SetPlayerDetectionStatus (Utilities|Struct|MakePlayerDetectionStatus false 0 "0.000000,0.000000,0.000000" 0.0))
  (Variables|Default|SetTackling false))

(event EventBeginPlay
  ;[1 1 1] BeginPlay Actions
  (|CallParentFunction)
  (Variables|Default|SetCurrentNode (Variables|Default|GetStartingNode))
  (bind _asenemy_aicontroller_aic (Utilities|Casting|CastToEnemy_AIController_AIC (Pawn|GetController)))
  (Variables|Default|SetAI_Controller _asenemy_aicontroller_aic)
  (CallFunction|SetBehaviour (Variables|Default|GetDefaultBehaviour))
  (Variables|Default|SetStartingTransform (Transformation|GetActorTransform))
  (Variables|Default|SetHealth 0.1)
  (Variables|Default|SetPlayerDetectionStatus (Utilities|Struct|MakePlayerDetectionStatus false 0 "0.000000,0.000000,0.000000" 0.0))
  (Variables|Default|SetTackling false))

(event EventTick
  (params (DeltaSeconds :type Float%20%28single-precision%29))
  (bind _canseeplayer (CallFunction|CanSeePlayer))
  (bind _returnvalue (Transformation|GetActorLocation))
  (bind _returnvalue_2 (Transformation|GetActorLocation))
  (bind _returnvalue_3 (+ _returnvalue_2 "0.000000,0.000000,-25.000000"))
  (bind _returnvalue_4 (+ _returnvalue "0.000000,0.000000,55.000000"))
  ;[1 1 1] Tick Actions
  (|CallParentFunction DeltaSeconds)
  (Utilities|FlowControl|Sequence
    (:then_0
      (if (not (Variables|Default|GetTackling))
        ;;[0 0 0] Player Detection System
        ;;;[1 1 1] Upper Box Trace for Standing Player
        (bind _outhit (Collision|BoxTraceByChannel _returnvalue_4 (+ _returnvalue_4 (Math|Vector|MakeVector (* (Variables|Default|GetLookDistance) (Math|Float|SelectFloat 1.0 -1.0 (CallFunction|IsFacingRight))) 0.0 0.0)) "25.000000,25.000000,25.000000" "0, 0, 0" "TraceTypeQuery1" false 0 "None"))
        ;;;[1 1 1] Lower Box Trace for Crouching Player
        (bind _outhit_2 (Collision|BoxTraceByChannel _returnvalue_3 (+ _returnvalue_3 (Math|Vector|MakeVector (* (Variables|Default|GetLookDistance) (Math|Float|SelectFloat 1.0 -1.0 (CallFunction|IsFacingRight))) 0.0 0.0)) "25.000000,25.000000,50.000000" "0, 0, 0" "TraceTypeQuery1" false 0 "None"))
        (if (.isPlayer (CallFunction|CheckBoxResultsforPlayer _outhit _outhit_2))
          (if _canseeplayer
            ;;;[1 1 1] No Change in Detection Status
            (Variables|Default|SetPlayerDetectionStatus (Utilities|Struct|MakePlayerDetectionStatus (.playerinsight (Variables|Default|GetPlayerDetectionStatus)) (.lastspottedplayer (Variables|Default|GetPlayerDetectionStatus)) (.lastspottedlocation (Variables|Default|GetPlayerDetectionStatus)) (+ (.timesincelastupdate (Variables|Default|GetPlayerDetectionStatus)) (Utilities|Time|GetWorldDeltaSeconds))) :!label _label)
            (else
              (|PlayerSpottedActions)
              (CallFunction|PlayerSeen (.PlayerCharacter (CallFunction|CheckBoxResultsforPlayer _outhit _outhit_2)))))
          (elif _canseeplayer
            (|PlayerLostActions)
            (CallFunction|PlayerLost)
            (else
              (goto _label))))))
    (:then_2
      ;;[0 0 0] Tackling Target Updates
      (if (Variables|Default|GetTackling)
        (|TackleTargetUpdates)))))

(event EventDie
  (Collision|SetCollisionResponsetoChannel (Variables|Character|GetMesh) "ECC_Pawn" "ECR_Ignore")
  (Collision|SetCollisionEnabled (Variables|Default|GetCapsuleComponent) "NoCollision")
  (Collision|SetCollisionEnabled (Variables|Default|GetMeshForDistanceFields) "NoCollision"))

(fn ConstructionScript
  (|CallParentFunction)
  (if (Variables|Default|GethasGun)
    (bind _returnvalue (AddComponent|AddSkeletalMeshComponent false))
    (bind _output_get (Variables|Default|SetGunMesh _returnvalue))
    (Transformation|AttachComponentToComponent _output_get (Variables|Character|GetMesh) "GunSocket" "SnapToTarget" "SnapToTarget" "SnapToTarget" true)
    (Components|SkeletalMesh|SetSkeletalMeshAsset (Variables|Default|GetGunMesh) "/Game/PGTemplate/Blueprints/Characters/Enemy/PrototypeWeaponsPack/Mesh/PistolFiring.PistolFiring")
    (Transformation|AttachComponentToComponent (Variables|Default|GetPistolFire_NS) (Variables|Default|GetGunMesh) "MuzzleFlash" "SnapToTarget" "SnapToTarget" "SnapToTarget" true)))

(fn IsFacingTowardsPlayer
  (return (< (Math|Vector|DotProduct (Transformation|GetActorForwardVector (Game|GetPlayerCharacter 0)) (Transformation|GetActorForwardVector)) 0.0)))

(fn PlayerSeen
  (params (SeenPlayer :type BP%20Player%20Character%20Object%20Reference))
  (Variables|Default|SetPlayerDetectionStatus (Utilities|Struct|MakePlayerDetectionStatus true SeenPlayer (Transformation|GetActorLocation SeenPlayer) 0.0))
  (Default|PlayerSpotted (Variables|Default|GetAI_Controller) SeenPlayer)
  (return))

(fn PlayerLost
  (Variables|Default|SetPlayerDetectionStatus (Utilities|Struct|MakePlayerDetectionStatus false (.lastspottedplayer (Variables|Default|GetPlayerDetectionStatus)) (.lastspottedlocation (Variables|Default|GetPlayerDetectionStatus)) 0.0)))

(fn CanSeePlayer
  (return (.playerinsight (Variables|Default|GetPlayerDetectionStatus))))

(fn CheckBoxResultsforPlayer
  (params (UpperBoxResult :type Hit%20Result%20Structure) (LowerBoxResult :type Hit%20Result%20Structure))
  (bind _asbp_player_character (Utilities|Casting|CastToBP_PlayerCharacter (.hitactor UpperBoxResult))
    (:then
      (return true _asbp_player_character))
    (:CastFailed
      (bind _asbp_player_character_2 (Utilities|Casting|CastToBP_PlayerCharacter (.hitactor LowerBoxResult))
        (:then
          (return true _asbp_player_character_2))
        (:CastFailed
          (return false 0))))))

(fn CurrentPatrolNode
  (bind _gamemoderef (Variables|Default|GetGameModeREF))
  (bind _patrolroute (Variables|Default|GetPatrolRoute))
  (bind _currentnode (Variables|Default|GetCurrentNode))
  (bind _returnvalue (Math|Conversions|ToFloat(Integer) _patrolroute))
  (bind _returnvalue_2 (Math|Conversions|ToFloat(Integer) _currentnode))
  (bind _patrolnodes (Variables|/Game/PGTemplate/Blueprints/Core/BP_PlatformGame_GameMode.BP_PlatformGame_GameMode_C|GetPatrolNodes _gamemoderef))
  (bind (_value _returnvalue_3) (Utilities|Map|Find _patrolnodes (Math|Vector2D|MakeVector2D _returnvalue _returnvalue_2)))
  (return _value _returnvalue_3))

(fn NextNode
  (bind _currentnode (Variables|Default|GetCurrentNode))
  (bind _returnvalue (+ _currentnode 1))
  (if (.ReturnValue (Utilities|Map|Find (Variables|/Game/PGTemplate/Blueprints/Core/BP_PlatformGame_GameMode.BP_PlatformGame_GameMode_C|GetPatrolNodes (Variables|Default|GetGameModeREF)) (Math|Vector2D|MakeVector2D (Math|Conversions|ToFloat(Integer) (Variables|Default|GetPatrolRoute)) (Math|Conversions|ToFloat(Integer) _returnvalue))))
    (return _returnvalue)
    (else
      (return 0))))

(fn PlayRandomIdleAnim
  (if (not (Variables|Default|GetTackling))
    (bind _returnvalue (Animation|PlayAnimMontage (.OutItem (Utilities|Array|Random (Variables|Default|GetIdleAnims))) 1.0 "None"))
    (return _returnvalue)))

(fn SetBehaviour
  (params (BehaviourState :type EnemyBehaviourState%20Enum :default "NewEnumerator0"))
  (bind _output_get (Variables|Default|SetBehaviourState BehaviourState))
  (Default|SetBehaviour (Variables|Default|GetAI_Controller) _output_get)
  (CallFunction|SetDesiredMovementGait (.Value (Utilities|Map|Find (Variables|Default|GetBehaviourGates) (Variables|Default|GetBehaviourState))))
  (Animation|StopAnimMontage 0))

(event Custom|PatrolNodeReached
  (Variables|Default|SetCurrentNode (CallFunction|NextNode))
  (Utilities|FlowControl|DoOnce false) ; enters at Reset
)

(event Custom|RestartIdleAnim
  (Utilities|FlowControl|DoOnce false) ; enters at Reset
)

(event Custom|DoneChasing
  (Utilities|FlowControl|DoOnce false) ; enters at Reset
)