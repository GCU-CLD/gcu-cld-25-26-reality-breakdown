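; Player camera manager for the platformer template, driving a fixed-rotation side-on camera that follows the player character.
; Each update eases the offset toward the current behaviour's gait-based horizontal lead and depth, flipping the lead with facing, with optional per-axis and in-air vertical tracking.
; It snaps into place on start or reset, and the character can force a lerped offset.
; FadeIn and FadeOut use a timeline to drive a post-process material parameter.
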(event Custom|RefreshPlayerPawn
  (bind _asbp_platform_game_character (Utilities|Casting|CastToBP_PlatformGameCharacter (Game|Player|GetPlayerPawn 0)))
  (bind _output_get (Variables|Default|SetPlayerPawn _asbp_platform_game_character))
  (Variables|Default|SetTrackedActor _output_get)
  (Variables|Default|SetLastOffset (- (Camera|GetCameraLocation) (Transformation|GetActorLocation _output_get)))
  (Variables|Default|SetInitialRun true))

(event Custom|FadeOut
  (params (FadeTime :type Float%20%28double-precision%29))
  (bind _dynamicpostprocessmaterial (Variables|Default|GetDynamicPostProcessMaterial))
  (Components|Timeline|SetPlayRate (Variables|Default|GetFade) (/ 1.0 FadeTime))
  (bind _fadealpha (Timeline|Fade PlayFromStart)
    (:Update
      (Utilities|IsValid _dynamicpostprocessmaterial
        (:Is%20Valid
          (Rendering|Material|SetScalarParameterValue _dynamicpostprocessmaterial "FadeAmount" _fadealpha :!class /Script/Engine.MaterialInstanceDynamic))))))

(event Custom|FadeIn
  (params (FadeTime :type Float%20%28double-precision%29))
  (bind _dynamicpostprocessmaterial (Variables|Default|GetDynamicPostProcessMaterial))
  (Components|Timeline|SetPlayRate (Variables|Default|GetFade) (/ 1.0 FadeTime))
  (bind _fadealpha (Timeline|Fade ReverseFromEnd)
    (:Update
      (Utilities|IsValid _dynamicpostprocessmaterial
        (:Is%20Valid
          (Rendering|Material|SetScalarParameterValue _dynamicpostprocessmaterial "FadeAmount" _fadealpha :!class /Script/Engine.MaterialInstanceDynamic))))))

(event EventBeginPlay
  (bind _returnvalue (Rendering|Material|CreateDynamicMaterialInstance "/Game/PGTemplate/Blueprints/Characters/Player/PP_HighlightSystem/PP_Outliner_M.PP_Outliner_M" "None" "None" :!class /Script/Engine.KismetMaterialLibrary))
  (Variables|Default|SetDynamicPostProcessMaterial _returnvalue)
  (bind _asbp_platform_game_character (Utilities|Casting|CastToBP_PlatformGameCharacter (Game|Player|GetPlayerPawn 0)))
  (bind _output_get (Variables|Default|SetPlayerPawn _asbp_platform_game_character))
  (Variables|Default|SetTrackedActor _output_get)
  (Variables|Default|SetLastOffset (- (Camera|GetCameraLocation) (Transformation|GetActorLocation _output_get)))
  (Variables|Default|SetInitialRun true))

(event EventOnReset
  (Utilities|FlowControl|DelayUntilNextTick)
  (Variables|Default|SetInitialRun true)
  (bind _asbp_platform_game_character (Utilities|Casting|CastToBP_PlatformGameCharacter (Game|Player|GetPlayerPawn 0)))
  (bind _output_get (Variables|Default|SetPlayerPawn _asbp_platform_game_character))
  (Variables|Default|SetTrackedActor _output_get)
  (Variables|Default|SetLastOffset (- (Camera|GetCameraLocation) (Transformation|GetActorLocation _output_get)))
  (Variables|Default|SetInitialRun true))

(event EventTick
  (params (DeltaSeconds :type Float%20%28single-precision%29)))

(fn ConstructionScript)

(fn BlueprintUpdateCamera
  (params (CameraTarget :type Actor%20Object%20Reference))
  (bind _returnvalue (Camera|GetCameraLocation))
  (bind _returnvalue_2 (Utilities|Time|GetWorldDeltaSeconds))
  (bind _returnvalue_3 (Camera|GetCameraLocation))
  (bind _currentbehaviour (Variables|Default|GetCurrentBehaviour))
  (bind _playerpawn (Variables|Default|GetPlayerPawn))
  (bind _currentbehaviour_2 (Variables|Default|GetCurrentBehaviour))
  (bind _trackedactor (Variables|Default|GetTrackedActor))
  (bind _playerpawn_2 (Variables|Default|GetPlayerPawn))
  (bind _currentbehaviour_3 (Variables|Default|GetCurrentBehaviour))
  (bind _playerpawn_3 (Variables|Default|GetPlayerPawn))
  (bind _currentbehaviour_4 (Variables|Default|GetCurrentBehaviour))
  (bind (_gaitbyspeed _gaitbypreference) (Default|GetCurrentGait _playerpawn))
  (bind _returnvalue_4 (Transformation|GetActorLocation _trackedactor))
  (bind _returnvalue_5 (Transformation|GetActorLocation _playerpawn_3))
  (bind _forcedcameraoffset (Variables|/Game/PGTemplate/Blueprints/Characters/Core/BP_PlatformGameCharacter.BP_PlatformGameCharacter_C|GetForcedCameraOffset _playerpawn_2))
  (bind _returnvalue_6 (- _returnvalue _returnvalue_4))
  (bind _returnvalue_7 (- _returnvalue_3 _returnvalue_5))
  (Utilities|IsValid _playerpawn_2
    (:Is%20Valid
      _)
    (:Is%20Not%20Valid
      (Development|PrintString "PlauerPawn not valid!")
      (CallFunction|RefreshPlayerPawn)))
  (if (Variables|/Game/PGTemplate/Blueprints/Characters/Core/BP_PlatformGameCharacter.BP_PlatformGameCharacter_C|GetForceCameraOffset _playerpawn_2)
    (Variables|Default|SetLastOffset _forcedcameraoffset)
    (bind _output_get (Variables|Default|SetLastPosition (Math|Vector|Lerp(Vector) (Variables|Default|GetLastPosition) (+ (Transformation|GetActorLocation (Variables|Default|GetTrackedActor)) _forcedcameraoffset) (* (Utilities|Time|GetWorldDeltaSeconds) (Variables|/Game/PGTemplate/Blueprints/Characters/Core/BP_PlatformGameCharacter.BP_PlatformGameCharacter_C|GetForcedCameraOffsetLerp _playerpawn_2)))))
    (return _output_get "0.000000,-90.000000,0.000000" 9e+01 (not (Variables|Default|GetOverrideCamera)))
    (else
      ;[1 1 1] Grab current Gait
      (if (Utilities|Enum|NotEqual(Enum) _gaitbyspeed "NewEnumerator0")
        (Variables|Default|SetCurrentPlayerGait _gaitbypreference))
      ;[1 1 1] Snap Camera into place on initial setup
      (if (Variables|Default|GetInitialRun)
        (Variables|Default|SetInitialRun false)
        (Variables|Default|SetOverrideCamera false)
        (bind _output_get_2 (Variables|Default|SetLastOffset (Math|Vector|MakeVector (.Value (Utilities|Map|Find (.horizontalleadbygait _currentbehaviour_4) "NewEnumerator2")) (.Value (Utilities|Map|Find (.depthbygait _currentbehaviour_4) "NewEnumerator2")) (Variables|Default|GetVerticalLead))))
        (bind _output_get_3 (Variables|Default|SetLastPosition (+ (Transformation|GetActorLocation (Variables|Default|GetTrackedActor)) _output_get_2)))
        (return _output_get_3 "0.000000,-90.000000,0.000000" (Camera|GetFOVAngle) (not (Variables|Default|GetOverrideCamera)))
        (else
          ;[1 1 1] Apply Offset to Player Position
          (bind _output_get_4 (Variables|Default|SetLastOffset (Math|Vector|MakeVector (Math|Float|SelectFloat (Math|Float|Lerp (.x (Variables|Default|GetLastOffset)) (* (.Value (Utilities|Map|Find (.horizontalleadbygait _currentbehaviour_2) (Variables|Default|GetCurrentPlayerGait))) (Math|Float|SelectFloat -1.0 1.0 (> (Math|Float|Absolute(Float) (.yaw (Transformation|GetActorRotation (Variables|Default|GetPlayerPawn)))) 0.0))) (* (.horizontallerp _currentbehaviour) _returnvalue_2)) (.x _returnvalue_6) (.updatehorizontal _currentbehaviour_3)) (Math|Float|SelectFloat (Math|Float|Lerp (.y (Variables|Default|GetLastOffset)) (.Value (Utilities|Map|Find (.depthbygait _currentbehaviour_2) (Variables|Default|GetCurrentPlayerGait))) (* (.depthlerp _currentbehaviour) _returnvalue_2)) (.y _returnvalue_6) (.updatedepth _currentbehaviour_3)) (Math|Float|Lerp (.z _returnvalue_7) (Math|Float|SelectFloat (.verticallead _currentbehaviour_2) (.z _returnvalue_7) (CallFunction|ShouldTrackPlayerZ)) (* (.verticallerp _currentbehaviour) _returnvalue_2)))))
          (bind _output_get_5 (Variables|Default|SetLastPosition (+ (Transformation|GetActorLocation (Variables|Default|GetTrackedActor)) _output_get_4)))
          (return _output_get_5 "0.000000,-90.000000,0.000000" 9e+01 (not (Variables|Default|GetOverrideCamera))))))))

(fn ShouldTrackPlayerZ
  (bind _currentbehaviour (Variables|Default|GetCurrentBehaviour))
  (bind _playerpawn (Variables|Default|GetPlayerPawn))
  (bind _charactermovement (Variables|/Script/Engine.Character|GetCharacterMovement _playerpawn))
  (bind _returnvalue (AI|Components|NavMovement|IsFalling _charactermovement))
  (return (and (or (not _returnvalue) (and _returnvalue (.trackinair _currentbehaviour))) (.updatevertical _currentbehaviour))))